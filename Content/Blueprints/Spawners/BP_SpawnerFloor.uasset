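; BP_SpawnerFloor is a child spawner that lays a row of floor tiles along X and recycles them as an endless floor.
; On BeginPlay it spawns the required count, takes tile size from the first tile's bounds and chains each behind RearTile.
; Tiles hitting bounds move to the rear after a brief delay instead of respawning.
; The game mode points update there currently multiplies by zero, adding nothing.
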(event EventBeginPlay
  (|CallParentFunction)
  (for _index (range 0 (Variables|Default|GetActorsRequiredCount))
    (if (== _index 0)
      ;[1 1 1] Fiirst tile
      (bind _returnvalue (CallFunction|SpawnActor))
      (Variables|Default|SetRearTile _returnvalue)
      (Variables|Default|SetTileSize (* (.x (.BoxExtent (Collision|GetActorBounds _returnvalue false))) 2.0))
      (Transformation|SetActorLocation (Variables|Default|GetRearTile) (Transformation|GetActorLocation) false false)
      (else
        ;[1 1 1] Spawn all other tiles
        (bind _returnvalue_2 (CallFunction|SpawnActor))
        (Transformation|SetActorLocation _returnvalue_2 (Math|Vector|MakeVector (+ (.x (Transformation|GetActorLocation (Variables|Default|GetRearTile))) (Variables|Default|GetTileSize)) (.y (Transformation|GetActorLocation (Variables|Default|GetRearTile))) 0.0) false false)
        (Variables|Default|SetRearTile _returnvalue_2)
        (Development|PrintString "NextTile")))))

(event EventSpawnedActorHitBounds
  (params (OutOfBoundsActor :type Actor%20Object%20Reference))
  (Utilities|FlowControl|Delay 0.01)
  (Transformation|SetActorLocation OutOfBoundsActor (Math|Vector|MakeVector (+ (.x (Transformation|GetActorLocation (Variables|Default|GetRearTile))) (Variables|Default|GetTileSize)) (.y (Transformation|GetActorLocation (Variables|Default|GetRearTile))) (.z (Transformation|GetActorLocation (Variables|Default|GetRearTile)))) false false)
  (Variables|Default|SetRearTile OutOfBoundsActor)
  (bind _asbp_game_mode_base (Utilities|Casting|CastToBP_GameModeBase (Game|GetGameMode)))
  (bind _output_get (Variables|/Game/Blueprints/Game/BP_GameModeBase.BP_GameModeBase_C|SetPoints _asbp_game_mode_base (+ (Variables|/Game/Blueprints/Game/BP_GameModeBase.BP_GameModeBase_C|GetPoints _asbp_game_mode_base) (* (Variables|/Game/Blueprints/Game/BP_GameModeBase.BP_GameModeBase_C|GetPointsMultiplier _asbp_game_mode_base) 0))))
  (Development|PrintString (Utilities|String|ToString(Integer) _output_get)))

(fn ConstructionScript
  (|CallParentFunction))

(fn SpawnActor
  (bind _returnvalue (|CallParentFunction))
  (return _returnvalue))
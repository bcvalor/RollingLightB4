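; Obstacle spawner that places obstacles at its own location at random intervals during play.
; On BeginPlay it caches the level manager, then a self-rescheduling event waits a random delay, spawns through the parent class's SpawnActor and repeats while the level is playing.
; Spawned actors reported out of bounds are destroyed.
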(event Custom|LineUpNextObstacleSpawn
  (Utilities|FlowControl|Delay (Math|Random|RandomFloatinRange (Variables|Default|GetMinDelay) (Variables|Default|GetMaxDelay)))
  (CallFunction|PlaceObstacle)
  (if (Variables|/Game/Blueprints/Game/BP_LevelManager.BP_LevelManager_C|GetbIsPlaying (Variables|Default|GetLevelManagerRef))
    (CallFunction|LineupNextObstacleSpawn)))

(event EventBeginPlay
  (bind (_levelmanager _levelmanagerfound) (CallFunction|GetLevelManager))
  (if _levelmanagerfound
    (Variables|Default|SetLevelManagerRef _levelmanager)
    (CallFunction|LineupNextObstacleSpawn)))

(event EventSpawnedActorHitBounds
  (params (OutOfBoundsActor :type Actor%20Object%20Reference))
  ;[1 1 1] When out of bounds, destroy actor
  (Actor|DestroyActor OutOfBoundsActor))

(fn ConstructionScript
  (|CallParentFunction))

(fn PlaceObstacle
  (bind _returnvalue (CallFunction|SpawnActor))
  (Transformation|SetActorLocation _returnvalue (Transformation|GetActorLocation) false false))

(fn SpawnActor
  (bind _returnvalue (|CallParentFunction))
  (return _returnvalue))

(fn ReturnParent
  (return 0))

(fn SetParent
  (params (Parent :type BP%20Spawner%20Base%20Object%20Reference))
  (return false))
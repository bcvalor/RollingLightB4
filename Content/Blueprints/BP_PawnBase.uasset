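; Base player pawn for a lane-based game, sidestepping between lanes on Left and Right input while the level is playing.
; On BeginPlay it reads lane count and width from the Level Manager and finds the camera tagged EndCam.
; Timelines lerp Y from the current position toward the next lane, blocking input until finished.
; HitObstacle blends the view to that camera and toggles Player visibility.
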(event EventBeginPlay
  (CallFunction|Initialize))

(event Input|ActionEvents|InputActionLeft
  (params (Key :type Key%20Structure))
  (bind _returnvalue (Transformation|GetActorLocation))
  (:Pressed
    (if (Variables|/Game/Blueprints/Game/BP_LevelManager.BP_LevelManager_C|GetbIsPlaying (Variables|Default|GetLevelManagerRef))
      ;[1 1 1] Check if we are on the left or not
      (if (not (== (Variables|Default|GetCurrentLane) 1))
        (if (not (Variables|Default|GetbMoving))
          (Variables|Default|SetbMoving true)
          ;[1 1 1] Determine which lane to travel to
          (Variables|Default|SetTargetPosition (- (.y (Transformation|GetActorLocation)) (Variables|Default|GetLaneWidth)))
          (bind _lefttrack (Timeline|MoveLeft PlayFromStart)
            (:Update
              (Transformation|SetActorLocation (Math|Vector|MakeVector (.x _returnvalue) (Math|Float|Lerp (.y _returnvalue) (Variables|Default|GetTargetPosition) _lefttrack) (.z _returnvalue)) false false))
            (:Finished
              (Variables|Default|SetbMoving false)
              (Math|Integer|DecrementInt (Variables|Default|GetCurrentLane)))))))))

(event Input|ActionEvents|InputActionRight
  (params (Key :type Key%20Structure))
  (bind _returnvalue (Transformation|GetActorLocation))
  (:Pressed
    (if (Variables|/Game/Blueprints/Game/BP_LevelManager.BP_LevelManager_C|GetbIsPlaying (Variables|Default|GetLevelManagerRef))
      ;[1 1 1] Check if we are on the right
      (if (not (== (Variables|Default|GetCurrentLane) (Variables|/Game/Blueprints/Game/BP_LevelManager.BP_LevelManager_C|GetNumOfLanes (Variables|Default|GetLevelManagerRef))))
        (if (not (Variables|Default|GetbMoving))
          (Variables|Default|SetbMoving true)
          ;[1 1 1] Determine which lane to travel to
          (Variables|Default|SetTargetPosition (+ (.y (Transformation|GetActorLocation)) (Variables|Default|GetLaneWidth)))
          (bind _righttrack (Timeline|RightTimeline PlayFromStart)
            (:Update
              (Transformation|SetActorLocation (Math|Vector|MakeVector (.x _returnvalue) (Math|Float|Lerp (.y _returnvalue) (Variables|Default|GetTargetPosition) _righttrack) (.z _returnvalue)) false false))
            (:Finished
              (Variables|Default|SetbMoving false)
              (Math|Integer|IncrementInt (Variables|Default|GetCurrentLane)))))))))

(fn ConstructionScript)

(fn Initialize
  (bind (_levelmanager _levelmanagerfound) (CallFunction|GetLevelManager))
  (if _levelmanagerfound
    (Variables|Default|SetLevelManagerRef _levelmanager)
    (Variables|Default|SetCurrentLane (/ (Variables|/Game/Blueprints/Game/BP_LevelManager.BP_LevelManager_C|GetNumOfLanes (Variables|Default|GetLevelManagerRef)) 2))
    (Variables|Default|SetLaneWidth (Variables|/Game/Blueprints/Game/BP_LevelManager.BP_LevelManager_C|GetLaneWidth (Variables|Default|GetLevelManagerRef)))
    (bind _outactors (Actor|GetAllActorswithTag "EndCam"))
    (Variables|Default|SetEndCamera (Utilities|Array|Get(acopy) _outactors))
    (else
      (Development|PrintString "All maps need a Level Manager!"))))

(fn HitObstacle
  (Game|Player|SetViewTargetwithBlend (Game|GetPlayerController 0) (Variables|Default|GetEndCamera) 1.2 "VTBlend_Linear" 0.0 false)
  (Rendering|ToggleVisibility (Variables|Default|GetPlayer) false))
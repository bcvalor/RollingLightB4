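; Level manager actor that runs the game flow from main menu to game over and polices the out-of-bounds area.
; BeginPlay opens the main menu with a self reference, while StartGame and GameOver toggle play state, input mode and cursor, with GameOver also zeroing level speed and showing its screen.
; A construction-configured LevelBounds box asks overlapping actors for their parent, then notifies that parent of the hit.
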(event OnComponentBeginOverlap(LevelBounds)
  (params (OverlappedComponent :type Primitive%20Component%20Object%20Reference) (OtherActor :type Actor%20Object%20Reference) (OtherComp :type Primitive%20Component%20Object%20Reference) (OtherBodyIndex :type Integer) (bFromSweep :type Boolean) (SweepResult :type Hit%20Result%20Structure%20%28by%20ref%29))
  (bind _parent (Class|BPISpawnable|ReturnParent(Message) OtherActor))
  (Utilities|IsValid _parent
    (:Is%20Valid
      (Default|SpawnedActorHitBounds _parent OtherActor))
    (:Is%20Not%20Valid
      (Development|PrintString "No actor returning to parent in Level Manager!"))))

(event EventBeginPlay
  (bind _returnvalue (UserInterface|CreateWidget "/Game/RollingFiles/UI/MainMenu/WBP_MainMenu.WBP_MainMenu_C" 0 (Variables|Default|GetPlayerInfo) self))
  (UserInterface|Viewport|AddtoViewport _returnvalue 0))

(fn ConstructionScript
  (bind _levelbounds (Variables|Default|GetLevelBounds))
  (Components|Box|SetBoxExtent _levelbounds (Variables|Default|GetOutOfBoundsBoxScale) true)
  (Transformation|SetWorldLocation _levelbounds (Variables|Default|GetOutOfBoundsBoxLocation) false false))

(fn GameOver
  (bind _returnvalue (Game|GetPlayerController 0))
  (Variables|Default|SetLevelSpeed 0.0)
  (Variables|Default|SetbIsPlaying false)
  (Viewport|RemoveAllWidgets)
  (bind _returnvalue_2 (UserInterface|CreateWidget "/Game/RollingFiles/UI/EndGame/WBP_GameOverScreen.WBP_GameOverScreen_C"))
  (UserInterface|Viewport|AddtoViewport _returnvalue_2 0)
  (Input|SetInputModeUIOnly _returnvalue 0 "DoNotLock")
  (Variables|/Script/Engine.PlayerController|SetbShowMouseCursor _returnvalue true))

(fn StartGame
  (bind _returnvalue (Game|GetPlayerController 0))
  (Variables|Default|SetbIsPlaying true)
  (Input|SetInputModeGameOnly _returnvalue)
  (Variables|/Script/Engine.PlayerController|SetbShowMouseCursor _returnvalue false))

(fn ReturnParent
  (return 0))

(fn SetParent
  (params (Parent :type BP%20Spawner%20Base%20Object%20Reference))
  (return false))
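; BP_MagnetPickup is a power-up pickup that turns on the character's magnet effect for a few seconds.
; On overlap with a ThirdPersonCharacter, it sets MagnetActive on that character and hides its mesh, leaving collision untouched.
; After a delay it clears the flag on player 0's character, plays a sound and destroys itself, printing debug messages at both ends.
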(event EventBeginPlay)

(event Collision|EventActorBeginOverlap
  (params (OtherActor :type Actor%20Object%20Reference))
  (bind _asthird_person_character (Utilities|Casting|CastToThirdPersonCharacter OtherActor))
  (Variables|/Game/RollingFiles/Blueprints/ThirdPersonCharacter.ThirdPersonCharacter_C|SetMagnetActive _asthird_person_character true)
  (Development|PrintString "Magnet Active")
  (Rendering|SetVisibility (Variables|Default|GetStaticMesh) false false)
  (Utilities|FlowControl|Delay 5.0)
  (bind _asthird_person_character_2 (Utilities|Casting|CastToThirdPersonCharacter (Game|GetPlayerCharacter 0)))
  (Variables|/Game/RollingFiles/Blueprints/ThirdPersonCharacter.ThirdPersonCharacter_C|SetMagnetActive _asthird_person_character_2 false)
  (Audio|PlaySound2D "/Game/Magic_Spells_1/General/cue/buff_up_attack__2__Cue.buff_up_attack__2__Cue" 1.0 1.0 0.0 0 0)
  (Development|PrintString "Magnet Inactive")
  (Actor|DestroyActor))

(event EventTick
  (params (DeltaSeconds :type Float%20%28single-precision%29)))

(fn ConstructionScript)
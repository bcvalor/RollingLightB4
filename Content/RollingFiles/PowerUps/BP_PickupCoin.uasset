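; Coin pickup that adds to the GameInfoInstance coin count, plays a sound and destroys itself.
; Touching the mesh collects it unless already used, also raising the character's level up to a cap of 4 and calling GrowthCheck.
; With the character's magnet active, the outer sphere counts the coin immediately without raising the level, then a timeline and VInterpTo pull it toward the player before delayed destruction.
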(event OnComponentBeginOverlap(Sphere)
  (params (OverlappedComponent :type Primitive%20Component%20Object%20Reference) (OtherActor :type Actor%20Object%20Reference) (OtherComp :type Primitive%20Component%20Object%20Reference) (OtherBodyIndex :type Integer) (bFromSweep :type Boolean) (SweepResult :type Hit%20Result%20Structure%20%28by%20ref%29))
  (bind _asthird_person_character (Utilities|Casting|CastToThirdPersonCharacter OtherActor))
  (if (Variables|/Game/RollingFiles/Blueprints/ThirdPersonCharacter.ThirdPersonCharacter_C|GetMagnetActive _asthird_person_character)
    (Utilities|FlowControl|Sequence
      (:then_0
        (bind _asgame_info_instance (Utilities|Casting|CastToGameInfoInstance (Game|GetGameInstance)))
        (Math|Integer|IncrementInt (Variables|/Game/RollingFiles/Blueprints/GameInfoInstance.GameInfoInstance_C|GetCurrentCoins _asgame_info_instance)
          (:%20%20
            (Variables|Default|SetUsedObject true)
            (Audio|PlaySound2D "/Game/RollingFiles/SFX/Pickup_SFX.Pickup_SFX" 1.0 1.0 0.0 0 0)
            (Utilities|FlowControl|Delay 1.0)
            (Actor|DestroyActor)
            (Default|GrowthCheck (Variables|Default|GetCharacterRef)))))
      (:then_1
        (bind _slide (Timeline|CoinSlide PlayFromStart)
          (:Update
            (Transformation|SetActorLocation (+ _slide (Math|Interpolation|VInterpTo (.Location (Math|Transform|BreakTransform (Transformation|GetActorTransform))) (Transformation|GetActorLocation (Game|GetPlayerCharacter 0)) (Utilities|Time|GetWorldDeltaSeconds) 15.0)) false false)))))))

(event OnComponentBeginOverlap(StaticMesh)
  (params (OverlappedComponent :type Primitive%20Component%20Object%20Reference) (OtherActor :type Actor%20Object%20Reference) (OtherComp :type Primitive%20Component%20Object%20Reference) (OtherBodyIndex :type Integer) (bFromSweep :type Boolean) (SweepResult :type Hit%20Result%20Structure%20%28by%20ref%29))
  (bind _asthird_person_character (Utilities|Casting|CastToThirdPersonCharacter OtherActor))
  (Variables|Default|SetCharacterRef _asthird_person_character)
  (bind _asgame_info_instance (Utilities|Casting|CastToGameInfoInstance (Game|GetGameInstance)))
  (if (not (Variables|Default|GetUsedObject))
    (Variables|/Game/RollingFiles/Blueprints/GameInfoInstance.GameInfoInstance_C|SetCurrentCoins _asgame_info_instance (+ (Variables|/Game/RollingFiles/Blueprints/GameInfoInstance.GameInfoInstance_C|GetCurrentCoins _asgame_info_instance) 1))
    (Audio|PlaySound2D "/Game/RollingFiles/SFX/Pickup_SFX.Pickup_SFX" 1.0 1.0 0.0 0 0)
    (Actor|DestroyActor)
    (if (< (Variables|/Game/RollingFiles/Blueprints/ThirdPersonCharacter.ThirdPersonCharacter_C|GetCurrentLVL _asthird_person_character) 4)
      (bind _output_get (Variables|/Game/RollingFiles/Blueprints/ThirdPersonCharacter.ThirdPersonCharacter_C|SetCurrentLVL (Variables|Default|GetCharacterRef) (+ (Variables|/Game/RollingFiles/Blueprints/ThirdPersonCharacter.ThirdPersonCharacter_C|GetCurrentLVL _asthird_person_character) 1)))
      (Variables|/Game/RollingFiles/Blueprints/ThirdPersonCharacter.ThirdPersonCharacter_C|SetPreviousLVL (Variables|Default|GetCharacterRef) (- _output_get 1))
      (Development|PrintString (Utilities|String|ToString(Integer) _output_get))
      (Default|GrowthCheck (Variables|Default|GetCharacterRef)))))

(event EventBeginPlay)

(event Collision|EventActorBeginOverlap
  (params (OtherActor :type Actor%20Object%20Reference)))

(event EventTick
  (params (DeltaSeconds :type Float%20%28single-precision%29)))

(fn ConstructionScript)
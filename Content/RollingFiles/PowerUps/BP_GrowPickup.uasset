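; BP_GrowPickup is a power-up pickup that temporarily makes the ThirdPersonCharacter larger.
; On overlap it calls the character's ShouldGrow, plays a buff sound and hides its mesh.
; After a fixed delay it calls ShouldShrink on player character 0, replays the sound, prints a status message and destroys itself.
; Collision stays active while hidden, so nothing in this graph blocks repeat overlaps during the delay.
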(event EventBeginPlay)

(event Collision|EventActorBeginOverlap
  (params (OtherActor :type Actor%20Object%20Reference))
  (bind _asthird_person_character (Utilities|Casting|CastToThirdPersonCharacter OtherActor))
  (Default|ShouldGrow _asthird_person_character)
  (Audio|PlaySound2D "/Game/Magic_Spells_1/General/cue/buff_up_attack__2__Cue.buff_up_attack__2__Cue" 1.0 1.0 0.0 0 0)
  (Rendering|SetVisibility (Variables|Default|GetStaticMesh) false false)
  (Utilities|FlowControl|Delay 5.0)
  (bind _asthird_person_character_2 (Utilities|Casting|CastToThirdPersonCharacter (Game|GetPlayerCharacter 0)))
  (Default|ShouldShrink _asthird_person_character_2)
  (Audio|PlaySound2D "/Game/Magic_Spells_1/General/cue/buff_up_attack__2__Cue.buff_up_attack__2__Cue" 1.0 1.0 0.0 0 0)
  (Development|PrintString "Super Size Inactive")
  (Actor|DestroyActor))

(event EventTick
  (params (DeltaSeconds :type Float%20%28single-precision%29)))

(fn ConstructionScript)
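; BP_BasicObstacle is an obstacle that penalizes the ThirdPersonCharacter when it overlaps the actor.
; On overlap it kills the character through DeathFunction if CurrentLVL is one or lower.
; Otherwise it calls the character's ShrinkCheck, then after a short delay decrements CurrentLVL, prints the new value and plays a fireball contact sound.
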(event EventBeginPlay)

(event Collision|EventActorBeginOverlap
  (params (OtherActor :type Actor%20Object%20Reference))
  (bind _asthird_person_character (Utilities|Casting|CastToThirdPersonCharacter OtherActor))
  (Variables|Default|SetCharacterRef _asthird_person_character)
  (if (<= (Variables|/Game/RollingFiles/Blueprints/ThirdPersonCharacter.ThirdPersonCharacter_C|GetCurrentLVL (Variables|Default|GetCharacterRef)) 1)
    (Default|DeathFunction (Variables|Default|GetCharacterRef))
    (else
      (Default|ShrinkCheck (Variables|Default|GetCharacterRef))
      ;[1 1 1] If not lowest level, decrement level
      (Utilities|FlowControl|Delay 0.2)
      (bind _output_get (Variables|/Game/RollingFiles/Blueprints/ThirdPersonCharacter.ThirdPersonCharacter_C|SetCurrentLVL (Variables|Default|GetCharacterRef) (- (Variables|/Game/RollingFiles/Blueprints/ThirdPersonCharacter.ThirdPersonCharacter_C|GetCurrentLVL (Variables|Default|GetCharacterRef)) 1)))
      (Development|PrintString (Utilities|String|ToString(Integer) _output_get))
      (Audio|PlaySound2D "/Game/MagicSoundFX/MagicCue/FireballCue/Cue_Fireball_Contact_8_Cue.Cue_Fireball_Contact_8_Cue" 1.0 1.0 0.0 0 0))))

(event EventTick
  (params (DeltaSeconds :type Float%20%28single-precision%29)))

(fn ConstructionScript)
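; Side-to-side obstacle that slides a sphere back and forth and calls the death function on any ThirdPersonCharacter overlapping the actor.
; The construction script derives two endpoint transforms from the actor's placement using fixed world-space offsets, separated along Y.
; From BeginPlay, LiftTimeline lerps the sphere from the end transform to the start, then reverses on each finish to loop indefinitely.
; Some disconnected movement nodes remain in both graphs.
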(event Custom|Forward
  (bind (_direction _lerptime) (Timeline|LiftTimeline PlayFromStart)
    (:Update
      (Transformation|SetWorldTransform (Variables|Default|GetBasicSphere) (Math|Transform|Lerp(Transform) (Variables|Default|GetEndTransform) (Variables|Default|GetStartTransform) _lerptime) false false))
    (:Finished
      (switch Utilities|FlowControl|Switch|SwitchonETimelineDirection _direction
        (:Forward
          (CallFunction|Backward))
        (:Backward
          (CallFunction|Forward))))))

(event Custom|Backward
  (bind (_direction _lerptime) (Timeline|LiftTimeline ReverseFromEnd)
    (:Update
      (Transformation|SetWorldTransform (Variables|Default|GetBasicSphere) (Math|Transform|Lerp(Transform) (Variables|Default|GetEndTransform) (Variables|Default|GetStartTransform) _lerptime) false false))
    (:Finished
      (switch Utilities|FlowControl|Switch|SwitchonETimelineDirection _direction
        (:Forward
          (CallFunction|Backward))
        (:Backward
          (CallFunction|Forward))))))

(event EventBeginPlay
  (bind (_direction _lerptime) (Timeline|LiftTimeline Play)
    (:Update
      (Transformation|SetWorldTransform (Variables|Default|GetBasicSphere) (Math|Transform|Lerp(Transform) (Variables|Default|GetEndTransform) (Variables|Default|GetStartTransform) _lerptime) false false))
    (:Finished
      (switch Utilities|FlowControl|Switch|SwitchonETimelineDirection _direction
        (:Forward
          (CallFunction|Backward))
        (:Backward
          (CallFunction|Forward))))))

(event Collision|EventActorBeginOverlap
  (params (OtherActor :type Actor%20Object%20Reference))
  (bind _asthird_person_character (Utilities|Casting|CastToThirdPersonCharacter OtherActor))
  (Default|DeathFunction _asthird_person_character))

(fn ConstructionScript
  (bind _returnvalue (Transformation|GetActorTransform))
  (bind (_location _rotation _scale) (Math|Transform|BreakTransform _returnvalue))
  (bind _returnvalue_2 (+ _location "0.000000,-50.000000,50.000000"))
  (bind _returnvalue_3 (Math|Transform|MakeTransform _returnvalue_2 _rotation _scale))
  (bind (_location_2 _rotation_2 _scale_2) (Math|Transform|BreakTransform _returnvalue_3))
  (Variables|Default|SetStartTransform _returnvalue_3)
  (Variables|Default|SetEndTransform (Math|Transform|MakeTransform (+ _location_2 "0.000000,300.000000,0.000000") _rotation_2 _scale_2)))
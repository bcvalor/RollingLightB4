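; First tile of an endless-runner track, which advances the run when the player crosses its trigger box.
; The overlap has the game mode spawn a main tile, adds multiplied points, raises walk speed within a clamp, then destroys the tile after a delay.
; SpawnObstacles, uncalled here, fills three lanes with obstacles or pickups via separate random rolls.
; Boots or empty results skip later lanes, and the magnet range is inverted (Min 9.0).
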(event OnComponentBeginOverlap(Box)
  (params (OverlappedComponent :type Primitive%20Component%20Object%20Reference) (OtherActor :type Actor%20Object%20Reference) (OtherComp :type Primitive%20Component%20Object%20Reference) (OtherBodyIndex :type Integer) (bFromSweep :type Boolean) (SweepResult :type Hit%20Result%20Structure%20%28by%20ref%29))
  (Utilities|Casting|CastToThirdPersonCharacter OtherActor)
  (bind _asthird_person_game_mode (Utilities|Casting|CastToThirdPersonGameMode (Game|GetGameMode)))
  (Default|SpawnMainTile _asthird_person_game_mode)
  (bind _asthird_person_game_mode_2 (Utilities|Casting|CastToThirdPersonGameMode (Game|GetGameMode)))
  (bind _output_get (Variables|/Game/RollingFiles/Blueprints/ThirdPersonGameMode.ThirdPersonGameMode_C|SetPoints _asthird_person_game_mode_2 (+ (Variables|/Game/RollingFiles/Blueprints/ThirdPersonGameMode.ThirdPersonGameMode_C|GetPoints _asthird_person_game_mode_2) (* 1 (Variables|/Game/RollingFiles/Blueprints/ThirdPersonGameMode.ThirdPersonGameMode_C|GetPoints%20Multiplier _asthird_person_game_mode_2)))))
  (Development|PrintString (Utilities|String|ToString(Integer) _output_get))
  (bind _asthird_person_character (Utilities|Casting|CastToThirdPersonCharacter (Game|GetPlayerCharacter 0)))
  (Variables|/Script/Engine.CharacterMovementComponent|SetMaxWalkSpeed (Variables|/Script/Engine.Character|GetCharacterMovement _asthird_person_character) (Math|Float|Clamp(Float) (* (Variables|/Script/Engine.CharacterMovementComponent|GetMaxWalkSpeed (Variables|/Script/Engine.Character|GetCharacterMovement _asthird_person_character)) 1.01) 6e+02 1.2e+03))
  (Utilities|FlowControl|Delay 0.5)
  (Actor|DestroyActor))

(event EventBeginPlay)

(event Collision|EventActorBeginOverlap
  (params (OtherActor :type Actor%20Object%20Reference)))

(event EventTick
  (params (DeltaSeconds :type Float%20%28single-precision%29)))

(fn ConstructionScript)

(fn SpawnObstacles
  (bind _returnvalue (Math|Random|RandomFloatinRange 0.0 1.0))
  (bind _returnvalue_2 (Math|Random|RandomFloatinRange 0.0 1.0))
  (bind _returnvalue_3 (Math|Random|RandomFloatinRange 0.0 1.0))
  ;[1 1 1] Lane 0
  (if (Math|Float|InRange(Float) _returnvalue_2 0.0 0.4)
    (Game|SpawnActorfromClass "/Game/RollingFiles/Obstacles/BP_BasicObstacle.BP_BasicObstacle_C" (Transformation|GetWorldTransform (Variables|Default|GetLane0)) "Undefined" 0 0)
    ;[1 1 1] Lane 1
    (if (Math|Float|InRange(Float) _returnvalue_3 0.0 0.4) :!label _label
      (Game|SpawnActorfromClass "/Game/RollingFiles/Obstacles/BP_BasicObstacle.BP_BasicObstacle_C" (Transformation|GetWorldTransform (Variables|Default|GetLane1)) "Undefined" 0 0)
      ;[1 1 1] Lane 0
      (if (Math|Float|InRange(Float) _returnvalue 0.0 0.4) :!label _label_2
        (Game|SpawnActorfromClass "/Game/RollingFiles/Obstacles/BP_BasicObstacle.BP_BasicObstacle_C" (Transformation|GetWorldTransform (Variables|Default|GetLaneCenter)) "Undefined" 0 0)
        (elif (Math|Float|InRange(Float) _returnvalue 0.4 0.5)
          (Game|SpawnActorfromClass "/Game/RollingFiles/Obstacles/BP_ObstacleBox.BP_ObstacleBox_C" (Transformation|GetWorldTransform (Variables|Default|GetLaneCenter)) "Undefined" 0 0)
          (elif (Math|Float|InRange(Float) _returnvalue 0.5 0.9)
            (Game|SpawnActorfromClass "/Game/RollingFiles/PowerUps/BP_PickupCoin.BP_PickupCoin_C" (Transformation|GetWorldTransform (Variables|Default|GetLaneCenter)) "Undefined" 0 0)
            (elif (Math|Float|InRange(Float) _returnvalue 9.0 0.95)
              (Game|SpawnActorfromClass "/Game/RollingFiles/PowerUps/BP_MagnetPickup.BP_MagnetPickup_C" (Transformation|GetWorldTransform (Variables|Default|GetLaneCenter)) "Undefined" 0 0)
              (elif (Math|Float|InRange(Float) _returnvalue 0.95 1.0)
                (Game|SpawnActorfromClass "/Game/RollingFiles/PowerUps/BP_BootsPickup.BP_BootsPickup_C" (Transformation|GetWorldTransform (Variables|Default|GetLaneCenter)) "Undefined" 0 0))))))
      (elif (Math|Float|InRange(Float) _returnvalue_3 0.4 0.5)
        (Game|SpawnActorfromClass "/Game/RollingFiles/Obstacles/BP_ObstacleBox.BP_ObstacleBox_C" (Transformation|GetWorldTransform (Variables|Default|GetLane1)) "Undefined" 0 0)
        (goto _label_2)
        (elif (Math|Float|InRange(Float) _returnvalue_3 0.5 0.9)
          (Game|SpawnActorfromClass "/Game/RollingFiles/PowerUps/BP_PickupCoin.BP_PickupCoin_C" (Transformation|GetWorldTransform (Variables|Default|GetLane1)) "Undefined" 0 0)
          (goto _label_2)
          (elif (Math|Float|InRange(Float) _returnvalue_3 9.0 0.95)
            (Game|SpawnActorfromClass "/Game/RollingFiles/PowerUps/BP_MagnetPickup.BP_MagnetPickup_C" (Transformation|GetWorldTransform (Variables|Default|GetLane1)) "Undefined" 0 0)
            (goto _label_2)
            (elif (Math|Float|InRange(Float) _returnvalue_3 0.95 1.0)
              (Game|SpawnActorfromClass "/Game/RollingFiles/PowerUps/BP_BootsPickup.BP_BootsPickup_C" (Transformation|GetWorldTransform (Variables|Default|GetLane1)) "Undefined" 0 0))))))
    (elif (Math|Float|InRange(Float) _returnvalue_2 0.4 0.5)
      (Game|SpawnActorfromClass "/Game/RollingFiles/Obstacles/BP_ObstacleBox.BP_ObstacleBox_C" (Transformation|GetWorldTransform (Variables|Default|GetLane0)) "Undefined" 0 0)
      (goto _label)
      (elif (Math|Float|InRange(Float) _returnvalue_2 0.5 0.9)
        (Game|SpawnActorfromClass "/Game/RollingFiles/PowerUps/BP_PickupCoin.BP_PickupCoin_C" (Transformation|GetWorldTransform (Variables|Default|GetLane0)) "Undefined" 0 0)
        (goto _label)
        (elif (Math|Float|InRange(Float) _returnvalue_2 9.0 0.95)
          (Game|SpawnActorfromClass "/Game/RollingFiles/PowerUps/BP_MagnetPickup.BP_MagnetPickup_C" (Transformation|GetWorldTransform (Variables|Default|GetLane0)) "Undefined" 0 0)
          (goto _label)
          (elif (Math|Float|InRange(Float) _returnvalue_2 0.95 1.0)
            (Game|SpawnActorfromClass "/Game/RollingFiles/PowerUps/BP_BootsPickup.BP_BootsPickup_C" (Transformation|GetWorldTransform (Variables|Default|GetLane0)) "Undefined" 0 0)))))))
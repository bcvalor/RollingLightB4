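; Endless-runner floor tile that populates itself with an obstacle or pickup and keeps the track going.
; On BeginPlay, SpawnObstacles picks one of three lanes, then rolls a fresh random number per spawn check, cycling to another lane until something spawns.
; When the character overlaps Box, it has the GameMode spawn the next tile, adds multiplied points, raises walk speed within a clamp, and destroys itself after a short delay.
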(event OnComponentBeginOverlap(Box)
  (params (OverlappedComponent :type Primitive%20Component%20Object%20Reference) (OtherActor :type Actor%20Object%20Reference) (OtherComp :type Primitive%20Component%20Object%20Reference) (OtherBodyIndex :type Integer) (bFromSweep :type Boolean) (SweepResult :type Hit%20Result%20Structure%20%28by%20ref%29))
  (Utilities|Casting|CastToThirdPersonCharacter OtherActor)
  (bind _asthird_person_game_mode (Utilities|Casting|CastToThirdPersonGameMode (Game|GetGameMode)))
  (Default|SpawnMainTile _asthird_person_game_mode)
  (Utilities|Casting|CastToGameInfoInstance (Game|GetGameInstance))
  (bind _asthird_person_game_mode_2 (Utilities|Casting|CastToThirdPersonGameMode (Game|GetGameMode)))
  (bind _output_get (Variables|/Game/RollingFiles/Blueprints/ThirdPersonGameMode.ThirdPersonGameMode_C|SetPoints _asthird_person_game_mode_2 (+ (Variables|/Game/RollingFiles/Blueprints/ThirdPersonGameMode.ThirdPersonGameMode_C|GetPoints _asthird_person_game_mode_2) (* 1 (Variables|/Game/RollingFiles/Blueprints/ThirdPersonGameMode.ThirdPersonGameMode_C|GetPoints%20Multiplier _asthird_person_game_mode_2)))))
  (Development|PrintString (Utilities|String|ToString(Integer) _output_get))
  (bind _asthird_person_character (Utilities|Casting|CastToThirdPersonCharacter (Game|GetPlayerCharacter 0)))
  (Variables|/Script/Engine.CharacterMovementComponent|SetMaxWalkSpeed (Variables|/Script/Engine.Character|GetCharacterMovement _asthird_person_character) (Math|Float|Clamp(Float) (* (Variables|/Script/Engine.CharacterMovementComponent|GetMaxWalkSpeed (Variables|/Script/Engine.Character|GetCharacterMovement _asthird_person_character)) 1.01) 6e+02 1.2e+03))
  (Utilities|FlowControl|Delay 0.5)
  (Actor|DestroyActor))

(event EventBeginPlay
  (CallFunction|SpawnObstacles))

(event Collision|EventActorBeginOverlap
  (params (OtherActor :type Actor%20Object%20Reference)))

(event EventTick
  (params (DeltaSeconds :type Float%20%28single-precision%29)))

(fn ConstructionScript)

(fn SpawnObstacles
  (bind _returnvalue (Math|Random|RandomFloatinRange 0.0 1.0))
  (bind _returnvalue_2 (Math|Random|RandomFloatinRange 0.0 1.0))
  (bind _returnvalue_3 (Math|Random|RandomFloatinRange 0.0 1.0))
  (bind _lane1 (Variables|Default|GetLane1))
  (bind _lane1_2 (Variables|Default|GetLane1))
  (bind _lane1_3 (Variables|Default|GetLane1))
  (bind _lane0 (Variables|Default|GetLane0))
  (bind _lane0_2 (Variables|Default|GetLane0))
  (bind _lane0_3 (Variables|Default|GetLane0))
  (bind _returnvalue_4 (Transformation|GetWorldTransform _lane1))
  (bind _returnvalue_5 (Transformation|GetWorldTransform _lane1_2))
  (bind _returnvalue_6 (Transformation|GetWorldTransform _lane1_3))
  (bind _returnvalue_7 (Transformation|GetWorldTransform _lane0))
  (bind _returnvalue_8 (Transformation|GetWorldTransform _lane0_2))
  (bind _returnvalue_9 (Transformation|GetWorldTransform _lane0_3))
  (bind (_location _rotation _scale) (Math|Transform|BreakTransform _returnvalue_5))
  (bind (_location_2 _rotation_2 _scale_2) (Math|Transform|BreakTransform _returnvalue_6))
  (bind (_location_3 _rotation_3 _scale_3) (Math|Transform|BreakTransform _returnvalue_7))
  (bind (_location_4 _rotation_4 _scale_4) (Math|Transform|BreakTransform _returnvalue_8))
  (bind (_location_5 _rotation_5 _scale_5) (Math|Transform|BreakTransform _returnvalue_9))
  (bind (_location_6 _rotation_6 _scale_6) (Math|Transform|BreakTransform _returnvalue_4))
  (bind (_x _y _z) (Math|Vector|BreakVector _location))
  (bind (_x_2 _y_2) (Math|Vector|BreakVector _location_2))
  (bind (_x_3 _y_3 _z_2) (Math|Vector|BreakVector _location_3))
  (bind (_x_4 _y_4) (Math|Vector|BreakVector _location_4))
  (bind (_x_5 _y_5 _z_3) (Math|Vector|BreakVector _location_5))
  (bind (_x_6 _y_6 _z_4) (Math|Vector|BreakVector _location_6))
  (switch int (Math|Random|RandomIntegerinRange 0 2)
    (:0
      ;[1 1 1] Lane 1 - No Rotating
      (if (Math|Float|InRange(Float) _returnvalue 0.0 0.4) :!label _label
        (Game|SpawnActorfromClass "/Game/RollingFiles/Obstacles/BP_BasicObstacle.BP_BasicObstacle_C" (Math|Transform|MakeTransform (Math|Vector|MakeVector (Math|Random|RandomFloatinRange -1.5e+02 1.5e+02) _y _z) _rotation _scale) "Undefined" 0 0)
        (elif (Math|Float|InRange(Float) _returnvalue 0.4 0.6)
          (Game|SpawnActorfromClass "/Game/RollingFiles/Obstacles/BP_UpDownObstacle.BP_UpDownObstacle_C" (Math|Transform|MakeTransform (Math|Vector|MakeVector _x_2 _y_2 (Math|Random|RandomFloatinRange -1e+02 2e+02)) _rotation_2 _scale_2) "Undefined" 0 0)
          (elif (Math|Float|InRange(Float) _returnvalue 0.6 0.8)
            (Game|SpawnActorfromClass "/Game/RollingFiles/Obstacles/BP_Side2SideObstacle.BP_Side2SideObstacle_C" (Math|Transform|MakeTransform (Math|Vector|MakeVector _x_6 (Math|Random|RandomFloatinRange 2e+02 2.5e+02) _z_4) _rotation_6 _scale_6) "Undefined" 0 0)
            (else
              ;[1 1 1] Lane 1 PowerUps
              (if (Math|Float|InRange(Float) _returnvalue 0.8 0.9)
                (Game|SpawnActorfromClass "/Game/RollingFiles/PowerUps/BP_PickupCoin.BP_PickupCoin_C" (Transformation|GetWorldTransform (Variables|Default|GetLane1)) "Undefined" 0 0)
                (elif (Math|Float|InRange(Float) _returnvalue 0.9 0.95)
                  (Game|SpawnActorfromClass "/Game/RollingFiles/PowerUps/BP_BootsPickup.BP_BootsPickup_C" (Transformation|GetWorldTransform (Variables|Default|GetLane1)) "Undefined" 0 0)
                  (elif (Math|Float|InRange(Float) _returnvalue 0.95 1.0)
                    (Game|SpawnActorfromClass "/Game/RollingFiles/PowerUps/BP_MagnetPickup.BP_MagnetPickup_C" (Transformation|GetWorldTransform (Variables|Default|GetLane1)) "Undefined" 0 0)
                    (else
                      ;[1 1 1] Lane 0 - No Rotating
                      (if (Math|Float|InRange(Float) _returnvalue_3 0.0 0.4) :!label _label_2
                        (Game|SpawnActorfromClass "/Game/RollingFiles/Obstacles/BP_BasicObstacle.BP_BasicObstacle_C" (Math|Transform|MakeTransform (Math|Vector|MakeVector (Math|Random|RandomFloatinRange -1.5e+02 1.5e+02) _y_3 _z_2) _rotation_3 _scale_3) "Undefined" 0 0)
                        (elif (Math|Float|InRange(Float) _returnvalue_3 0.4 0.6)
                          (Game|SpawnActorfromClass "/Game/RollingFiles/Obstacles/BP_UpDownObstacle.BP_UpDownObstacle_C" (Math|Transform|MakeTransform (Math|Vector|MakeVector _x_4 _y_4 (Math|Random|RandomFloatinRange -1e+02 2e+02)) _rotation_4 _scale_4) "Undefined" 0 0)
                          (elif (Math|Float|InRange(Float) _returnvalue_3 0.6 0.8)
                            (Game|SpawnActorfromClass "/Game/RollingFiles/Obstacles/BP_Side2SideObstacle.BP_Side2SideObstacle_C" (Math|Transform|MakeTransform (Math|Vector|MakeVector _x_5 (Math|Random|RandomFloatinRange -4.5e+02 -4e+02) _z_3) _rotation_5 _scale_5) "Undefined" 0 0)
                            (else
                              ;[1 1 1] Lane 0 PowerUps
                              (if (Math|Float|InRange(Float) _returnvalue_3 0.8 0.9)
                                (Game|SpawnActorfromClass "/Game/RollingFiles/PowerUps/BP_PickupCoin.BP_PickupCoin_C" (Transformation|GetWorldTransform (Variables|Default|GetLane0)) "Undefined" 0 0)
                                (elif (Math|Float|InRange(Float) _returnvalue_3 0.9 0.95)
                                  (Game|SpawnActorfromClass "/Game/RollingFiles/PowerUps/BP_BootsPickup.BP_BootsPickup_C" (Transformation|GetWorldTransform (Variables|Default|GetLane0)) "Undefined" 0 0)
                                  (elif (Math|Float|InRange(Float) _returnvalue_3 0.95 1.0)
                                    (Game|SpawnActorfromClass "/Game/RollingFiles/PowerUps/BP_MagnetPickup.BP_MagnetPickup_C" (Transformation|GetWorldTransform (Variables|Default|GetLane0)) "Undefined" 0 0)
                                    (else
                                      ;[1 1 1] Lane 1
                                      (if (Math|Float|InRange(Float) _returnvalue_2 0.0 0.4) :!label _label_3
                                        (Game|SpawnActorfromClass "/Game/RollingFiles/Obstacles/BP_BasicObstacle.BP_BasicObstacle_C" (Transformation|GetWorldTransform (Variables|Default|GetLaneCenter)) "Undefined" 0 0)
                                        (elif (Math|Float|InRange(Float) _returnvalue_2 0.4 0.5)
                                          (Game|SpawnActorfromClass "/Game/RollingFiles/Obstacles/BP_RotatingObstacle.BP_RotatingObstacle_C" (Transformation|GetWorldTransform (Variables|Default|GetLaneCenter)) "Undefined" 0 0)
                                          (elif (Math|Float|InRange(Float) _returnvalue_2 0.5 0.9)
                                            (Game|SpawnActorfromClass "/Game/RollingFiles/PowerUps/BP_PickupCoin.BP_PickupCoin_C" (Transformation|GetWorldTransform (Variables|Default|GetLaneCenter)) "Undefined" 0 0)
                                            (elif (Math|Float|InRange(Float) _returnvalue_2 9.0 0.95)
                                              (Game|SpawnActorfromClass "/Game/RollingFiles/Obstacles/BP_UpDownObstacle.BP_UpDownObstacle_C" (Transformation|GetWorldTransform (Variables|Default|GetLaneCenter)) "Undefined" 0 0)
                                              (elif (Math|Float|InRange(Float) _returnvalue_2 0.95 1.0)
                                                (Game|SpawnActorfromClass "/Game/RollingFiles/PowerUps/BP_BootsPickup.BP_BootsPickup_C" (Transformation|GetWorldTransform (Variables|Default|GetLaneCenter)) "Undefined" 0 0)
                                                (else
                                                  (goto _label))))))))))))))))))))))))
    (:1
      (goto _label_3))
    (:2
      (goto _label_2))))

(fn RandomTransformX
  (params (Transform :type Transform))
  (bind (_location _rotation _scale) (Math|Transform|BreakTransform Transform))
  (bind (_x _y _z) (Math|Vector|BreakVector _location))
  (return (Math|Transform|MakeTransform (Math|Vector|MakeVector (Math|Random|RandomFloatinRange -1.5e+02 1.5e+02) _y _z) _rotation _scale)))